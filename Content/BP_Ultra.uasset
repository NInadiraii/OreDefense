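; BP_Ultra is an auto-firing attacker that shoots BP_Enemy actors with a bouncing shot.
; A looping timer calls Fire, which locks the nearest enemy within AttackRange and waits FireRate before damaging it, guarded by IsFiring.
; It then searches all enemies, primary included, for the one nearest the impact point, dealing half damage only if that differs from the primary target.
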(event Custom|Fire
  (if (not (Variables|Default|GetbIsFiring))
    (bind _outactors (Actor|GetAllActorsOfClass "/Game/BP_Enemy.BP_Enemy_C"))
    (if (<= (.Distance (Actor|FindNearestActor (Transformation|GetActorLocation) _outactors)) (Variables|Default|GetAttackRange))
      (bind _asbp_enemy (Utilities|Casting|CastToBP_Enemy (.ReturnValue (Actor|FindNearestActor (Transformation|GetActorLocation) _outactors))))
      (Utilities|IsValid _asbp_enemy
        (:Is%20Valid
          (Variables|Default|SetPrimaryTarget _asbp_enemy)
          (Variables|Default|SetbIsFiring true)
          (Development|PrintString "TARGET LOCKED")
          (Utilities|FlowControl|Delay (Variables|Default|GetFireRate))
          (Utilities|IsValid (Variables|Default|GetPrimaryTarget)
            (:Is%20Valid
              (Variables|Default|SetBounceOrigin (Transformation|GetActorLocation (Variables|Default|GetPrimaryTarget)))
              (Default|TakeDamage (Variables|Default|GetPrimaryTarget) (Variables|Default|GetAttackDamage))
              (Development|PrintString "SHOT FIRED")
              (bind _outactors_2 (Actor|GetAllActorsOfClass "/Game/BP_Enemy.BP_Enemy_C"))
              (bind _asbp_enemy_2 (Utilities|Casting|CastToBP_Enemy (.ReturnValue (Actor|FindNearestActor (Variables|Default|GetBounceOrigin) _outactors_2))))
              (if (!= _asbp_enemy_2 (Variables|Default|GetPrimaryTarget))
                (Default|TakeDamage _asbp_enemy_2 (/ (Variables|Default|GetAttackDamage) 2.0)))
              (Variables|Default|SetbIsFiring false))
            (:Is%20Not%20Valid
              (Variables|Default|SetbIsFiring false)))))
      (else
        (Variables|Default|SetbIsFiring false)))))

(event EventBeginPlay
  (Utilities|Time|SetTimerbyEvent (delegate Custom|Fire) (Variables|Default|GetFireRate) true))

(fn ConstructionScript)