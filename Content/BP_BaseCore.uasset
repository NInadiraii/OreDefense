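; BP_BaseCore is a destructible core actor whose destruction halts the game.
; A custom TakeDamage event subtracts the incoming value from CoreHP; at zero or below it flags IsDead and prints a destroyed message.
; It then adds a WBP_GameScreen widget to the viewport, pauses the game and sets mouse cursor visibility from the pause call's result.
; BeginPlay only reassigns CoreHP to itself.
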(event Custom|TakeDamage
  (params (NewParam :type Float%20%28double-precision%29))
  (Variables|Default|SetCoreHP (- (Variables|Default|GetCoreHP) NewParam))
  (if (<= (Variables|Default|GetCoreHP) 0.0)
    (Variables|Default|SetbIsDead true)
    (Development|PrintString "Core Destroyed")
    (bind _returnvalue (UserInterface|CreateWidget "/Game/WBP_GameScreen.WBP_GameScreen_C"))
    (UserInterface|Viewport|AddtoViewport _returnvalue 0)
    (bind _returnvalue_2 (Game|SetGamePaused true))
    (Variables|/Script/Engine.PlayerController|SetbShowMouseCursor (Game|GetPlayerController 0) _returnvalue_2)))

(event EventBeginPlay
  (Variables|Default|SetCoreHP (Variables|Default|GetCoreHP)))

(event Collision|EventActorBeginOverlap
  (params (OtherActor :type Actor%20Object%20Reference)))

(event EventTick
  (params (DeltaSeconds :type Float%20%28single-precision%29)))

(fn ConstructionScript)