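; Enemy actor that advances on a referenced Core, damages it on reaching close range and then destroys itself.
; Tick moves it straight toward the Core on the XY plane by offsetting its location at Movespeed, without sweep or pathfinding.
; TakeDamage lowers HP and updates its widget health bar.
; At zero HP it reports a random Coal, Iron or Copper drop to the GameInstance's HUD reference and destroys itself.
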(event Custom|TakeDamage
  (params (DamageAmount :type Float%20%28double-precision%29))
  (bind _output_get (Variables|Default|SetEnemy_HP (- (Variables|Default|GetEnemy_HP) DamageAmount)))
  (bind _aswbp_health_bar (Utilities|Casting|CastToWBP_HealthBar (UserInterface|GetUserWidgetObject (Variables|Default|GetWidget))))
  (Variables|/Game/WBP_HealthBar.WBP_HealthBar_C|SetHealthPercent _aswbp_health_bar (/ (Variables|Default|GetEnemy_HP) (Variables|Default|GetMaxEnemy_HP)))
  (if (<= _output_get 0.0)
    (bind _asbp_game_instance (Utilities|Casting|CastToBP_GameInstance (Game|GetGameInstance)))
    (Default|ReportDrop (Variables|/Game/BP_GameInstance.BP_GameInstance_C|GetHUDRef _asbp_game_instance) (Utilities|Select :Index (Math|Random|RandomIntegerinRange 0 2) :Option%200 "Coal" :Option%201 "Iron" :Option%202 "Copper"))
    (Actor|DestroyActor)))

(event EventBeginPlay)

(event Collision|EventActorBeginOverlap
  (params (OtherActor :type Actor%20Object%20Reference)))

(event EventTick
  (params (DeltaSeconds :type Float%20%28single-precision%29))
  (bind _returnvalue (Transformation|GetActorLocation))
  (bind _corereference (Variables|Default|GetCoreReference))
  (bind _returnvalue_2 (Transformation|GetActorLocation _corereference))
  (bind _returnvalue_3 (- _returnvalue_2 _returnvalue))
  (bind (_x _y) (Math|Vector|BreakVector _returnvalue_3))
  (Utilities|IsValid _corereference
    (:Is%20Valid
      (if (<= (Math|Vector|Distance(Vector) _returnvalue _returnvalue_2) 1e+02)
        (Default|TakeDamage (Variables|Default|GetCoreReference) (Variables|Default|GetDamage))
        (Actor|DestroyActor)
        (else
          (Transformation|AddActorWorldOffset (* (* (Math|Vector|Normalize (Math|Vector|MakeVector _x _y 0.0)) (Variables|Default|GetMovespeed)) DeltaSeconds)))))))

(fn ConstructionScript)