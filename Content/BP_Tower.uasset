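; BP_Tower is a tower that periodically damages nearby enemies.
; On BeginPlay it starts a looping timer at FireRate that calls FireAtTraget.
; Each call gathers every BP_Enemy in the level, applies AttackDamage to all within AttackRnage of the tower rather than a single target, and prints a debug "HIT" for each.
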(event Custom|FireAtTraget
  (bind _outactors (Actor|GetAllActorsOfClass "/Game/BP_Enemy.BP_Enemy_C"))
  (for _array_element _outactors
    (if (<= (Math|Vector|Distance(Vector) (Transformation|GetActorLocation _array_element) (Transformation|GetActorLocation)) (Variables|Default|GetAttack%20Rnage))
      (Default|TakeDamage _array_element (Variables|Default|GetAttack%20Damage))
      (Development|PrintString "HIT"))))

(event EventBeginPlay
  (Utilities|Time|SetTimerbyEvent (delegate Custom|FireAtTraget) (Variables|Default|GetFireRate) true))

(event Collision|EventActorBeginOverlap
  (params (OtherActor :type Actor%20Object%20Reference)))

(event EventTick
  (params (DeltaSeconds :type Float%20%28single-precision%29)))

(fn ConstructionScript)