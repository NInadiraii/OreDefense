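; Enemy spawner that creates BP_Enemy actors around the world origin and tracks waves toward a win screen.
; BeginPlay caches the first BP_BaseCore, starts a looping spawn timer and spawns immediately, passing the core to each enemy.
; Cosine and sine use separate random angles, so spawns scatter within a square rather than on a circle.
; NextWave, not called here, re-arms itself and, past MaxWaves, shows WBP_GameWin and pauses.
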(event Custom|SpawnEnemy
  (bind _returnvalue (Math|Random|RandomFloatinRange 0.0 3.6e+02))
  (Game|SpawnActorfromClass "/Game/BP_Enemy.BP_Enemy_C" (Math|Transform|MakeTransform (Math|Vector|MakeVector (* (Math|Trig|Cos(Degrees) _returnvalue) (Variables|Default|Getspawn%20radius)) (* (Math|Trig|Sin(Degrees) _returnvalue) (Variables|Default|Getspawn%20radius)) 1e+01)) "AlwaysSpawn" "MultiplyWithRoot" 0 (Variables|Default|GetCoreReference) 0))

(event Custom|NextWave
  (Utilities|Time|SetTimerbyEvent (delegate Custom|NextWave) 3e+01 true)
  (bind _output_get (Variables|Default|SetWaveNumber (+ (Variables|Default|GetWaveNumber) 1)))
  (if (> _output_get (Variables|Default|GetMaxWaves))
    (bind _returnvalue (UserInterface|CreateWidget "/Game/WBP_GameWin.WBP_GameWin_C"))
    (UserInterface|Viewport|AddtoViewport _returnvalue 0)
    (bind _returnvalue_2 (Game|SetGamePaused true))
    (Variables|/Script/Engine.PlayerController|SetbShowMouseCursor (Game|GetPlayerController 0) _returnvalue_2)))

(event EventBeginPlay
  (bind _returnvalue (Math|Random|RandomFloatinRange 0.0 3.6e+02))
  (bind _outactors (Actor|GetAllActorsOfClass "/Game/BP_BaseCore.BP_BaseCore_C"))
  (Variables|Default|SetCoreReference (Utilities|Array|Get(acopy) _outactors))
  (Utilities|Time|SetTimerbyEvent (delegate Custom|SpawnEnemy) (Variables|Default|GetSpawnInterval) true)
  (Game|SpawnActorfromClass "/Game/BP_Enemy.BP_Enemy_C" (Math|Transform|MakeTransform (Math|Vector|MakeVector (* (Math|Trig|Cos(Degrees) _returnvalue) (Variables|Default|Getspawn%20radius)) (* (Math|Trig|Sin(Degrees) _returnvalue) (Variables|Default|Getspawn%20radius)) 1e+01)) "AlwaysSpawn" "MultiplyWithRoot" 0 (Variables|Default|GetCoreReference) 0))

(event Collision|EventActorBeginOverlap
  (params (OtherActor :type Actor%20Object%20Reference)))

(event EventTick
  (params (DeltaSeconds :type Float%20%28single-precision%29)))

(fn ConstructionScript)